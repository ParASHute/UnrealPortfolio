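; BP_Boss is the Boss Bokoblin enemy, a child Blueprint driven by the Gameplay Ability System.
; BeginPlay attaches a spawned weapon, fills the hit montages and binds the HP bar to attribute changes.
; Damage and gameplay events for arrow hits, stun and Just Rush activate abilities by tag.
; Tick re-registers those event waits every frame and polls an attribute to trigger death, which disables collision and plays the death montage.
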(event Input|EnhancedActionEvents|EnhancedInputActionIA_Move
  (params (ActionValue :type Vector%202D%20Structure) (ElapsedSeconds :type Float%20%28double-precision%29) (TriggeredSeconds :type Float%20%28double-precision%29) (InputAction :type Input%20Action%20Object%20Reference :default "/Game/03_Characters/00_Link/Input/Actions/IA_Move.IA_Move"))
  (bind _returnvalue (Pawn|GetControlRotation :!class /Script/Engine.Pawn))
  (bind _returnvalue_2 (Math|Rotator|MakeRotator 0.0 0.0 (.yaw _returnvalue)))
  (Pawn|Input|AddMovementInput (Math|Vector|GetRightVector _returnvalue_2) (.x ActionValue) false) ; X
  (Pawn|Input|AddMovementInput (Math|Vector|GetForwardVector _returnvalue_2) (.y ActionValue) false) ; Y
)

(event EventBeginPlay
  (|CallParentFunction)
  (bind _returnvalue (Game|SpawnActorfromClass "/Game/02_Equpments/01_Monster/BP_BossWeapon.BP_BossWeapon_C" (Math|Transform|MakeTransform "0, 0, 0") "Undefined" "MultiplyWithRoot" 0 0))
  (Transformation|AttachComponentToComponent _returnvalue (Variables|Character|GetMesh) "b_MF_Weapon_R_Socket" "KeepRelative" "KeepRelative" "KeepRelative" true)
  (|ReSetMontage)
  (|Hp))

(event Collision|EventActorBeginOverlap
  (params (OtherActor :type Actor%20Object%20Reference))
  (|CallParentFunction OtherActor) ; 지금 이 노드는 비활성 상태입니다. \n핀을 끌어서 다른 노드를 연결하면 활성화됩니다.
)

(event EventTick
  (params (DeltaSeconds :type Float%20%28single-precision%29))
  (|Sturn)
  (|JustRush)
  (|ArrowHit)
  (|CheckDaeth (Variables|Default|GetAbilitySystemComponent)
    (:Death
      (|Death))))

(event Game|Damage|EventAnyDamage
  (params (Damage :type Float%20%28single-precision%29) (DamageType :type Damage%20Type%20Object%20Reference) (InstigatedBy :type Controller%20Object%20Reference) (DamageCauser :type Actor%20Object%20Reference))
  (|CallParentFunction Damage DamageType InstigatedBy DamageCauser)
  (Abilities|TryActivateAbilitiesbyTag (Variables|Default|GetAbilitySystemComponent) (GameplayTags|MakeLiteralGameplayTagContainer "(GameplayTags=((TagName=\"Monster.State.Damaged\")))") true))

(fn ConstructionScript
  (|CallParentFunction))