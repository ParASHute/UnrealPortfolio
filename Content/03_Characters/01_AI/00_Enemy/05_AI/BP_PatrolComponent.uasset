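; Patrol component for an enemy AI character that walks a target point along a PatrolPath spline.
; UpdateLocation writes the world location at the current Distance to the PatrolLocation blackboard key.
; Distance wraps at either spline end; open splines also set Reverse to false at both ends, so they never switch into reverse.
; CalculateDistance holds walk-speed times delta-time steps in both directions, but they are unconnected.
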(event Custom|Update%20Location
  (bind (__ ___2) (|CalculateDistance))
  (bind _patrolpath (Variables|Default|GetPatrolPath))
  (bind _spline (Variables|/Script/Portfolio.PatrolPath|GetSpline _patrolpath))
  (bind _returnvalue (Class|SplineComponent|IsClosedLoop _spline))
  (Utilities|IsValid (Variables|Default|GetPatrolPath)
    (:Is%20Valid
      (if (Variables|Default|GetReverse)
        (bind _output_get (Variables|Default|SetDistance __))
        (if (<= _output_get 0.0)
          (Variables|Default|SetDistance (Spline|GetSplineLength (Variables|/Script/Portfolio.PatrolPath|GetSpline (Variables|Default|GetPatrolPath))))
          (if _returnvalue
            _
            (else
              ;[1 1 1] 직선구간
              (Variables|Default|SetReverse false))))
        (else
          (bind _output_get_2 (Variables|Default|SetDistance ___2))
          (if (>= _output_get_2 (Spline|GetSplineLength (Variables|/Script/Portfolio.PatrolPath|GetSpline (Variables|Default|GetPatrolPath))))
            (Variables|Default|SetDistance 0.0)
            (if _returnvalue
              _
              (else
                (Variables|Default|SetReverse false))))))
      (bind _output_get_3 (Variables|Default|SetLocation (Spline|GetLocationatDistanceAlongSpline (Variables|/Script/Portfolio.PatrolPath|GetSpline (Variables|Default|GetPatrolPath)) (Variables|Default|GetDistance) "World")))
      (AI|Components|Blackboard|SetValueasVector (AI|GetBlackboard (Pawn|GetController (Variables|Default|GetOwnerCharacter))) (Utilities|Name|MakeLiteralName "PatrolLocation") _output_get_3))))

(event EventBeginPlay
  (bind _as캐릭터 (Utilities|Casting|CastToCharacter (Components|GetOwner)))
  (Variables|Default|SetOwnerCharacter _as캐릭터))