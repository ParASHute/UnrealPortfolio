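; Player character Link: handles movement, sword and bow combat, damage reactions and death.
; Enhanced Input drives movement, weapon swaps and tag-gated GAS abilities, with jump and attack becoming avoid and parry while guarding.
; Sword guard locks the camera onto a nearby I_LockOn actor found by sphere trace; drawing the bow also locks it.
; Tick updates lock-on and airtime, polls for death, and ends Just Rush slow-motion, which time-dilation compensation exempts Link from.
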(event Custom|LockOnTarget
  (bind _outhits (|ShootTrace))
  (|AddHittedActors _outhits
    (:then
      (|FindClosestAcotr
        (:Completed
          (|SetCarmera))))))

(event Custom|UnLockTarget
  (|TargetReset)
  (Variables|ForLockRatget|SetDistance 1e+07) ; ResetDistance
  (|UnlockCamera)
  (Variables|Default|SetAnimInstanceChange false))

(event EventTick
  (params (DeltaSeconds :type Float%20%28single-precision%29))
  (|Jumpping DeltaSeconds)
  (|JustRush)
  (|CheckLockTarget)
  (|CheckDaeth_2 (Variables|Default|GetAbilitySystemComponent))
  (|Death_2))

(event EventBeginPlay
  (|CallParentFunction)
  (Utilities|FlowControl|Sequence
    (:then_0
      (|AddInput))
    (:then_1
      (Variables|/Script/Engine.CharacterMovementComponent|SetMaxWalkSpeed (Variables|Character|GetCharacterMovement) 5e+02))))

(event Game|Damage|EventAnyDamage
  (params (Damage :type Float%20%28single-precision%29) (DamageType :type Damage%20Type%20Object%20Reference) (InstigatedBy :type Controller%20Object%20Reference) (DamageCauser :type Actor%20Object%20Reference))
  (|CallParentFunction Damage DamageType InstigatedBy DamageCauser)
  (Abilities|TryActivateAbilitiesbyTag (Variables|Default|GetAbilitySystemComponent) (GameplayTags|MakeLiteralGameplayTagContainer "(GameplayTags=((TagName=\"State.Damaged\")))") true))

(fn ConstructionScript
  (|CallParentFunction))

(fn SetJustRushTime
  (Utilities|Time|SetGlobalTimeDilation 0.3)
  (Variables|Default|SetCustomTimeDilation (/ 1.0 (Class|GameplayStatics|GetGlobalTimeDilation)))
  (Variables|Default|SetIsJusttime true))

(fn EndJustRush
  (Utilities|Time|SetGlobalTimeDilation 1.0)
  (Variables|Default|SetCustomTimeDilation (/ 1.0 (Class|GameplayStatics|GetGlobalTimeDilation)))
  (Variables|Default|SetIsJusttime false))

(event Input|EnhancedActionEvents|EnhancedInputActionIA_Jump
  (params (ActionValue :type Boolean) (ElapsedSeconds :type Float%20%28double-precision%29) (TriggeredSeconds :type Float%20%28double-precision%29) (InputAction :type Input%20Action%20Object%20Reference :default "/Game/03_Characters/00_Link/Input/Actions/IA_Jump.IA_Jump"))
  (:Started
    (if (GameplayTags|HasMatchingGameplayTag (Variables|Default|GetAbilitySystemComponent) "(TagName=\"Defence.Idle\")")
      (Abilities|TryActivateAbilitiesbyTag (Variables|Default|GetAbilitySystemComponent) (GameplayTags|MakeLiteralGameplayTagContainer "(GameplayTags=((TagName=\"Defence.Avoid\")))") true)
      (else
        (Character|Jump)))))

(event Input|EnhancedActionEvents|EnhancedInputActionIA_Look
  (params (ActionValue :type Vector%202D%20Structure) (ElapsedSeconds :type Float%20%28double-precision%29) (TriggeredSeconds :type Float%20%28double-precision%29) (InputAction :type Input%20Action%20Object%20Reference :default "/Game/03_Characters/00_Link/Input/Actions/IA_Look.IA_Look"))
  (Pawn|Input|AddControllerYawInput (.x ActionValue)) ; X
  (Pawn|Input|AddControllerPitchInput (.y ActionValue)) ; Y
)

(event Input|EnhancedActionEvents|EnhancedInputActionIA_Move
  (params (ActionValue :type Vector%202D%20Structure) (ElapsedSeconds :type Float%20%28double-precision%29) (TriggeredSeconds :type Float%20%28double-precision%29) (InputAction :type Input%20Action%20Object%20Reference :default "/Game/03_Characters/00_Link/Input/Actions/IA_Move.IA_Move"))
  (bind _returnvalue (Pawn|GetControlRotation :!class /Script/Engine.Pawn))
  (bind _returnvalue_2 (Math|Rotator|MakeRotator 0.0 0.0 (.yaw _returnvalue)))
  (Pawn|Input|AddMovementInput (Math|Vector|GetRightVector _returnvalue_2) (.x ActionValue) false) ; X
  (Pawn|Input|AddMovementInput (Math|Vector|GetForwardVector _returnvalue_2) (.y ActionValue) false) ; Y
)

(event Input|EnhancedActionEvents|EnhancedInputActionIA_Attack
  (params (ActionValue :type Boolean) (ElapsedSeconds :type Float%20%28double-precision%29) (TriggeredSeconds :type Float%20%28double-precision%29) (InputAction :type Input%20Action%20Object%20Reference :default "/Game/03_Characters/00_Link/Input/Actions/IA_Attack.IA_Attack"))
  (bind _abilitysystemcomponent (Variables|Default|GetAbilitySystemComponent))
  (bind _returnvalue (Class|AbilitySystemComponent|GetGameplayTagCount _abilitysystemcomponent "(TagName=\"Attack.DrawingBow\")"))
  (bind _returnvalue_2 (> _returnvalue 0))
  ;[1 1 1] Attack
  (:Started
    (if (> (Class|AbilitySystemComponent|GetGameplayTagCount (Variables|Default|GetAbilitySystemComponent) "(TagName=\"Defence.Idle\")") 0)
      (Variables|/Script/Portfolio.WeaponComponent|SetSwapping (Variables|Default|GetWeaponComponent) true)
      (Abilities|TryActivateAbilitiesbyTag (Variables|Default|GetAbilitySystemComponent) (GameplayTags|MakeLiteralGameplayTagContainer "(GameplayTags=((TagName=\"Defence.Parry\")))") true)
      (Utilities|FlowControl|Delay 0.2)
      (Variables|/Script/Portfolio.WeaponComponent|SetSwapping (Variables|Default|GetWeaponComponent) false)
      (elif (> (Class|AbilitySystemComponent|GetGameplayTagCount (Variables|Default|GetAbilitySystemComponent) "(TagName=\"State.ArmdBow\")") 0)
        (Variables|/Script/Portfolio.WeaponComponent|SetSwapping (Variables|Default|GetWeaponComponent) true)
        (Abilities|TryActivateAbilitiesbyTag (Variables|Default|GetAbilitySystemComponent) (GameplayTags|MakeLiteralGameplayTagContainer "(GameplayTags=((TagName=\"Attack\")))") true) ; 공격
        ;[1 1 1] CarmeraLock
        (if _returnvalue_2
          (Class|PortfolioCharacter|CameraLock _returnvalue_2)
          (Variables|Default|SetIsCarmeraLock _returnvalue_2))
        (else
          (Abilities|TryActivateAbilitiesbyTag (Variables|Default|GetAbilitySystemComponent) (GameplayTags|MakeLiteralGameplayTagContainer "(GameplayTags=((TagName=\"Attack\")))") true)))))
  (:Completed
    (if (> (Class|AbilitySystemComponent|GetGameplayTagCount (Variables|Default|GetAbilitySystemComponent) "(TagName=\"Attack.DrawingBow\")") 0)
      (Ability|SendGameplayEventtoActor self "(TagName=\"Attack.ShootArrow\")")
      (Class|PortfolioCharacter|CameraUnLock (not _returnvalue_2))
      (Variables|Default|SetIsCarmeraLock false)
      (Utilities|FlowControl|Delay 0.2)
      (Variables|/Script/Portfolio.WeaponComponent|SetSwapping (Variables|Default|GetWeaponComponent) false))))

(event Input|EnhancedActionEvents|EnhancedInputActionIA_EquipSword
  (params (ActionValue :type Boolean) (ElapsedSeconds :type Float%20%28double-precision%29) (TriggeredSeconds :type Float%20%28double-precision%29) (InputAction :type Input%20Action%20Object%20Reference :default "/Game/03_Characters/00_Link/Input/Actions/IA_EquipSword.IA_EquipSword"))
  (Class|PortfolioCharacter|RemoveLoosGamePlayTag self (GameplayTags|MakeLiteralGameplayTag "(TagName=\"State.ArmdBow\")"))
  (Class|WeaponComponent|SelectWeapon (Variables|Default|GetWeaponComponent) "Sword" true))

(event Input|EnhancedActionEvents|EnhancedInputActionIA_EquipBow
  (params (ActionValue :type Boolean) (ElapsedSeconds :type Float%20%28double-precision%29) (TriggeredSeconds :type Float%20%28double-precision%29) (InputAction :type Input%20Action%20Object%20Reference :default "/Game/03_Characters/00_Link/Input/Actions/IA_EquipBow.IA_EquipBow"))
  (Class|PortfolioCharacter|RemoveLoosGamePlayTag self (GameplayTags|MakeLiteralGameplayTag "(TagName=\"State.ArmdSwrod\")"))
  (Class|WeaponComponent|SelectWeapon (Variables|Default|GetWeaponComponent) "Bow" false))

(event Input|EnhancedActionEvents|EnhancedInputActionIA_Run
  (params (ActionValue :type Boolean) (ElapsedSeconds :type Float%20%28double-precision%29) (TriggeredSeconds :type Float%20%28double-precision%29) (InputAction :type Input%20Action%20Object%20Reference :default "/Game/03_Characters/00_Link/Input/Actions/IA_Run.IA_Run"))
  (bind _returnvalue (GameplayTags|MakeLiteralGameplayTag "(TagName=\"State.Run\")"))
  (bind _self self)
  (bind _charactermovement (Variables|Character|GetCharacterMovement))
  (bind _abilitysystemcomponent (Variables|Default|GetAbilitySystemComponent))
  (bind _abilitysystemcomponent_2 (Variables|Default|GetAbilitySystemComponent))
  (:Triggered
    (Variables|/Script/Engine.CharacterMovementComponent|SetMaxWalkSpeed _charactermovement 7.5e+02)
    (Class|PortfolioCharacter|AddLoosGamePlayTag _self _returnvalue)
    (if (> (Math|Vector|VectorLengthXY (Variables|/Script/Engine.MovementComponent|GetVelocity (Variables|Character|GetCharacterMovement))) 0.0)
      (GameplayEffects|RemoveActiveGameplayEffectbySourceEffect _abilitysystemcomponent_2 "/Game/03_Characters/00_Link/Ability/Move/GE_EndDssh.GE_EndDssh_C" 0 -1)
      (GameplayEffects|ApplyGameplayEffectToSelf :self _abilitysystemcomponent_2 :GameplayEffectClass "/Game/03_Characters/00_Link/Ability/Move/GE_Dssh.GE_Dssh_C")
      (else
        (GameplayEffects|RemoveActiveGameplayEffectbySourceEffect _abilitysystemcomponent_2 "/Game/03_Characters/00_Link/Ability/Move/GE_Dssh.GE_Dssh_C" 0 -1)
        (GameplayEffects|ApplyGameplayEffectToSelf :self _abilitysystemcomponent_2 :GameplayEffectClass "/Game/03_Characters/00_Link/Ability/Move/GE_EndDsshForTriggered.GE_EndDsshForTriggered_C"))))
  (:Completed
    (Variables|/Script/Engine.CharacterMovementComponent|SetMaxWalkSpeed _charactermovement 5e+02)
    (Class|PortfolioCharacter|RemoveLoosGamePlayTag _self _returnvalue)
    (GameplayEffects|RemoveActiveGameplayEffectbySourceEffect _abilitysystemcomponent "/Game/03_Characters/00_Link/Ability/Move/GE_Dssh.GE_Dssh_C" 0 -1)
    (GameplayEffects|ApplyGameplayEffectToSelf :self _abilitysystemcomponent :GameplayEffectClass "/Game/03_Characters/00_Link/Ability/Move/GE_EndDssh.GE_EndDssh_C")))

(event Input|EnhancedActionEvents|EnhancedInputActionIA_Defence
  (params (ActionValue :type Boolean) (ElapsedSeconds :type Float%20%28double-precision%29) (TriggeredSeconds :type Float%20%28double-precision%29) (InputAction :type Input%20Action%20Object%20Reference :default "/Game/03_Characters/00_Link/Input/Actions/IA_Defence.IA_Defence"))
  (:Started
    (if (> (Class|AbilitySystemComponent|GetGameplayTagCount (Variables|Default|GetAbilitySystemComponent) "(TagName=\"State.ArmdSwrod\")") 0)
      (Abilities|TryActivateAbilitiesbyTag (Variables|Default|GetAbilitySystemComponent) (GameplayTags|MakeLiteralGameplayTagContainer "(GameplayTags=((TagName=\"State.Defence\")))") true)
      (Variables|Default|SetAnimInstanceChange true)
      (if (not (Variables|ForLockRatget|GetTargetLock))
        (CallFunction|LockonTarget))))
  (:Completed
    (Variables|ForSheild|SetCancled true)
    (CallFunction|UnLockTarget)
    (Class|AbilitySystemComponent|InputCancel (Variables|Default|GetAbilitySystemComponent))))

(event Input|KeyboardEvents|LeftAlt
  (params (Key :type Key%20Structure))
  (bind _returnvalue (GameplayTags|MakeLiteralGameplayTag "(TagName=\"State.Burrow\")"))
  (bind _self self)
  (bind _charactermovement (Variables|Character|GetCharacterMovement))
  (:Pressed
    (Variables|/Script/Engine.CharacterMovementComponent|SetMaxWalkSpeed _charactermovement 125.0)
    (Class|PortfolioCharacter|AddLoosGamePlayTag _self _returnvalue))
  (:Released
    (Variables|/Script/Engine.CharacterMovementComponent|SetMaxWalkSpeed _charactermovement 5e+02)
    (Class|PortfolioCharacter|RemoveLoosGamePlayTag _self _returnvalue)))