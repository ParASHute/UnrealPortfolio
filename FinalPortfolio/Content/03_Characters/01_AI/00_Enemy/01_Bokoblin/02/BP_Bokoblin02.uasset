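; Archer Bokoblin enemy that spawns a BP_MonsterBow on its mesh socket and fires it through Gameplay Ability System tags.
; Shoot runs a delay-timed sequence: draw-arrow ability, bow montages, then a shoot gameplay event, with the camera socketed for the arrow trace.
; Damage activates the Damaged ability, and an attribute listener reveals and updates the HP bar.
; Stun, just-rush, arrow-hit and death-check calls sit in unconnected BeginPlay leftovers.
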(event Custom|Shoot
  ;[1 1 1] 플레이어 바라보기는 비헤이비어 트리에서 구현
  ; 에님 블프 사용 안하고 테그 따라 틱에서 계속 실행
  (|ShootBow))

(event EventBeginPlay
  (|CallParentFunction)
  (bind _returnvalue (Game|SpawnActorfromClass "/Game/02_Equpments/01_Monster/Bow/BP_MonsterBow.BP_MonsterBow_C" (Math|Transform|MakeTransform "0, 0, 0") "Undefined" "MultiplyWithRoot" 0 0))
  (bind _output_get (Variables|Default|SetBow _returnvalue))
  (Transformation|AttachComponentToComponent _output_get (Variables|Character|GetMesh) "Bow" "KeepRelative" "KeepRelative" "KeepRelative" true)
  ;[1 1 1] 라인트레이스가 손에서 나가기 때문에
  ; 카메라를 화살 위치에 붙임
  (Transformation|AttachComponentToComponent (Variables|Default|GetFollowCamera) (Variables|Character|GetMesh) "CarmeraSocket" "KeepRelative" "KeepRelative" "KeepRelative" true)
  (|ReSetMontage)
  (|Hp))

(event Collision|EventActorBeginOverlap
  (params (OtherActor :type Actor%20Object%20Reference))
  (|CallParentFunction OtherActor) ; 지금 이 노드는 비활성 상태입니다. \n핀을 끌어서 다른 노드를 연결하면 활성화됩니다.
)

(event EventTick
  (params (DeltaSeconds :type Float%20%28single-precision%29)))

(event Game|Damage|EventAnyDamage
  (params (Damage :type Float%20%28single-precision%29) (DamageType :type Damage%20Type%20Object%20Reference) (InstigatedBy :type Controller%20Object%20Reference) (DamageCauser :type Actor%20Object%20Reference))
  (|CallParentFunction Damage DamageType InstigatedBy DamageCauser)
  (Abilities|TryActivateAbilitiesbyTag (Variables|Default|GetAbilitySystemComponent) (GameplayTags|MakeLiteralGameplayTagContainer "(GameplayTags=((TagName=\"Monster.State.Damaged\")))") true))

(fn ConstructionScript
  (|CallParentFunction))